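; BP_MeteorSkill is a skill actor that runs the meteor spell's cast and spawn sequence at its own position.
; On BeginPlay a timeline feeds a cast-bar widget for two seconds, then the widget is removed and the player's casting flag clears.
; It spawns a circle and an overhead portal, with heights relative to the player, then drops in the meteor stone after a delay.
; Only the circle is destroyed here, after a further delay.
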(event `self.ReceiveBeginPlay`
  (bind _returnvalue (`self.K2_GetActorLocation`))
  (bind (_returnvalue_x _returnvalue_y _returnvalue_z) (`KismetMathLibrary.BreakVector` (`self.K2_GetActorLocation` (`GameplayStatics.GetPlayerCharacter` 0))))
  (bind _returnvalue_2 (`KismetMathLibrary.MakeVector` (.x _returnvalue) (.y _returnvalue) (+ _returnvalue_z 450.0)))
  (bind _returnvalue_3 (`KismetMathLibrary.MakeVector` (.x _returnvalue_2) (.y _returnvalue_2) (+ _returnvalue_z 420.0)))
  (bind _returnvalue_4 (`|CreateWidget` "/Game/LHW/ui/WBP_catingUi.WBP_catingUi_C"))
  (`UserWidget.AddToViewport` _returnvalue_4 0)
  (`|ExecutionSequence`
    (:`then_0`
      (bind (_direction `_새_트랙_0`) (`Timeline|bar delay`)
        (:`Update`
          (`/Engine/EditorBlueprintResources/StandardMacros.IsValid` _returnvalue_4
            (:`Is Valid`
              (set `/Game/LHW/ui/WBP_catingUi.SkillCastTime` `_새_트랙_0` _returnvalue_4))))))
    (:`then_1`
      (`KismetSystemLibrary.Delay` 2.0)
      (`Widget.RemoveFromParent` _returnvalue_4)
      (bind _asmyplayer_character (cast `/Game/LHW/BluePrint/MyplayerCharacter` (`GameplayStatics.GetPlayerCharacter` 0)))
      (set `/Game/LHW/BluePrint/MyplayerCharacter.isSkillCasting` false _asmyplayer_character)
      (bind _returnvalue_5 (`|SpawnActorFromClass` "/Game/LHW/Skill_Resouroes/Meteor/Meteor_circle.Meteor_circle_C" (`KismetMathLibrary.MakeTransform` (`KismetMathLibrary.MakeVector` (.x _returnvalue) (.y _returnvalue) (+ _returnvalue_z -70.0))) "Undefined" "MultiplyWithRoot" null null))
      (set `self.getMouseClick` _returnvalue_3)
      (`|SpawnActorFromClass` "/Game/LHW/Skill_Resouroes/Meteor/Meteor_portal.Meteor_portal_C" (`KismetMathLibrary.MakeTransform` _returnvalue_2 (struct) (0.8 0.8 0.8)) "Undefined" "MultiplyWithRoot" null null)
      (`KismetSystemLibrary.Delay` 1.0)
      (`|SpawnActorFromClass` "/Game/LHW/Skill_Resouroes/Meteor/Meteor_stone.Meteor_stone_C" (`KismetMathLibrary.MakeTransform` _returnvalue_3) "Undefined" "MultiplyWithRoot" null null)
      (`KismetSystemLibrary.Delay` 5.0)
      (`self.K2_DestroyActor` _returnvalue_5))))

(event `self.ReceiveTick`
  (params (DeltaSeconds :type "Float (single-precision)")))

(fn `UserConstructionScript`)