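; Player character Blueprint for mouse-aimed combat, with an icicle skill, a meteor skill and a normal projectile-style attack.
; E or R spawns area indicators, and left click casts at that area, removes them and starts a timer-based cooldown.
; Left click also turns the character to the cursor hit point and spawns normal attacks, gated by flags.
; Attacks halt movement and disable controller input, which Tick restores whenever IsSkillCasting is false.
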(event `InputAction|RightClick`
  (params (Key :type "Key Structure"))
  ; 스킬 취소
)

(event `Key|Escape`
  (params (Key :type "Key Structure"))
  ; 스킬 취소
  (:`Pressed`
    (set `self.SkillKey` "None")))

(event `InputAction|Skill`
  (params (Key :type "Key Structure"))
  ; 키보드 입력 이후
  (:`Pressed`
    (bind _output_get (set `self.SkillKey` Key))
    (if (`self.isClick`)
      (`|ExecutionSequence`
        (:`then_0`
          (if (== _output_get "E")
            (if (`self.IceCoolDown`)
              (set `self.SkillKey` "None" :!label _label)
              (else
                (set `self.onchageKey` 1)
                (set `self.SkilRange` (1.0 1.0 1.0))
                (set `self.isClick` false :!label _label_2)
                (bind _returnvalue (`|SpawnActorFromClass` "/Game/LHW/BluePrint/BP_AttackArea.BP_AttackArea_C" (`KismetMathLibrary.MakeTransform` (0.0 0.0 0.0)) "Undefined" "MultiplyWithRoot" null null))
                (bind _returnvalue_2 (`|SpawnActorFromClass` "/Game/LHW/BluePrint/BP_Magic_Area.BP_Magic_Area_C" (`KismetMathLibrary.MakeTransform` (0.0 0.0 0.0) (struct) (`self.SkilRange`)) "Undefined" "MultiplyWithRoot" null null))
                (`/Engine/EditorBlueprintResources/StandardMacros.IsValid` _returnvalue_2
                  (:`Is Valid`
                    (set `self.AttacAreaOb` _returnvalue_2)))))))
        (:`then_1`
          (if (== _output_get "R")
            (if (`self.MeteorCoolDown`)
              (goto _label)
              (else
                (set `self.onchageKey` 2)
                (set `self.SkilRange` (3.0 3.0 3.0))
                (goto _label_2)))))))))

(event `Key|LeftMouseButton`
  (params (Key :type "Key Structure"))
  (bind _skillkey (`self.SkillKey`))
  ; 마우스 클릭이후
  (:`Pressed`
    (if (`self.attackDelay`)
      (`self.CharacterfindMousePosition`))
    (`|ExecutionSequence`
      (:`then_0`
        (if (== _skillkey "E")
          (if (not (`self.IceCoolDown`))
            (set `self.onchageKey` 1)
            (set `self.isSkilAnim` true)
            (`self.Skill3`)
            (`/Engine/EditorBlueprintResources/StandardMacros.IsValid` (stale `InputAction|Skill` _returnvalue_2)
              (:`Is Valid`
                ; 파괴
                (`self.K2_DestroyActor` (stale `InputAction|Skill` _returnvalue_2))
                (`self.K2_DestroyActor` (stale `InputAction|Skill` _returnvalue))
                (set `self.isClick` true :!label _label_3))))))
      (:`then_1`
        (if (== _skillkey "R")
          (set `self.onchageKey` 2)
          (set `self.isSkilAnim` true)
          (`self.SpawnMeteor`)
          (`/Engine/EditorBlueprintResources/StandardMacros.IsValid` (stale `InputAction|Skill` _returnvalue_2)
            (:`Is Valid`
              (`self.K2_DestroyActor` (stale `InputAction|Skill` _returnvalue_2))
              (`self.K2_DestroyActor` (stale `InputAction|Skill` _returnvalue))
              (goto _label_3)))))
      (:`then_2`
        (if (== _skillkey "RightMouseButton")
          (set `self.onchageKey` 0)
          (set `self.SkillKey` "None")))
      (:`then_3`
        (if (and (`self.attackDelay`) (`self.asdnalsnd`))
          (`self.StopMovementPlayer`)
          (`self.normalAttact`)
          (`KismetSystemLibrary.Delay` 0.2)
          (`self.StartMovementPlayer`))))))

(event `self.ReceiveActorBeginOverlap`
  (params (OtherActor :type "Actor Object Reference")))

(event `InputAction|Space`
  (params (Key :type "Key Structure")))

(event `self.ReceiveTick`
  (params (DeltaSeconds :type "Float (single-precision)"))
  (if (not (`self.isSkillCasting`))
    (`self.StartMovementPlayer`)))

(fn `CharacterfindMousePosition`
  (bind _returnvalue (`KismetMathLibrary.FindLookAtRotation` (`self.K2_GetActorLocation`) (`self.MousePosition`)))
  (`self.getMousePosition`)
  (set `self.NewVar` _returnvalue)
  (`self.K2_SetActorRotation` _returnvalue))

(fn `CoolDownIce`
  (`KismetSystemLibrary.PrintString` "아이스에이지 쿨타운 끝" true true (struct :`R` 1.0 :`G` 0.956113 :`B` 0.286401 :`A` 1.0))
  (set `self.IceCoolDown` false))

(fn `CoolDownTeteor`
  (`KismetSystemLibrary.PrintString` "메테오 쿨타운 끝" true true (struct :`R` 1.0 :`G` 0.956113 :`B` 0.286401 :`A` 1.0))
  (set `self.MeteorCoolDown` false))

(fn `getMousePosition`
  (set `self.MousePosition` (`.ImpactPoint` (`GameplayStatics.BreakHitResult` (`PlayerController.GetHitResultUnderCursorByChannel` (`GameplayStatics.GetPlayerController` 0) "TraceTypeQuery1" true)))))

(fn `normalAttact`
  (bind _returnvalue (`self.K2_GetActorLocation`))
  (bind _returnvalue_2 (`GameplayStatics.GetPlayerCharacter` 0))
  (bind (_returnvalue_x _returnvalue_y) (`KismetMathLibrary.BreakVector` (+ (* (`self.GetActorForwardVector` _returnvalue_2) 200) (* (`self.GetActorUpVector` _returnvalue_2) 200) _returnvalue)))
  (`|SpawnActorFromClass` "/Game/LHW/Skill_Resouroes/NormalAttack/BP_NormalAttack.BP_NormalAttack_C" (`KismetMathLibrary.MakeTransform` (`KismetMathLibrary.MakeVector` _returnvalue_x _returnvalue_y (.z _returnvalue)) (`KismetMathLibrary.FindLookAtRotation` (`self.K2_GetActorLocation` (`GameplayStatics.GetPlayerCharacter` 0)) (`self.MousePosition`))) "Undefined" "MultiplyWithRoot" null null)
  (`self.K2_SetActorRotation` (`KismetMathLibrary.FindLookAtRotation` (`self.K2_GetActorLocation`) (`self.MousePosition`))))

(fn `Skill3`
  (bind _returnvalue (`self.K2_GetActorLocation` (`self.AttacAreaOb`)))
  (bind _returnvalue_2 (`|SpawnActorFromClass` "/Game/LHW/Skill_Resouroes/ice/BP_Icicle.BP_Icicle_C" (`KismetMathLibrary.MakeTransform` (+ (`self.K2_GetActorLocation`) (`KismetMathLibrary.MakeVector` (`KismetMathLibrary.Conv_Int64ToDouble` (* (`KismetMathLibrary.RandomInteger64InRange` -20 20) 10)) 0.0 200.0)) (struct) (0.5 0.5 0.5)) "Undefined" "OverrideRootScale" null null))
  (bind _output_get (set `self.SpawnedIceActor` _returnvalue_2))
  (set `/Game/LHW/Skill_Resouroes/ice/BP_Icicle.TargetLocation` _returnvalue _output_get)
  (`self.K2_SetActorRotation` _returnvalue_2 (`KismetMathLibrary.FindLookAtRotation` (`self.K2_GetActorLocation` _returnvalue_2) _returnvalue) false)
  (`self.StopMovementPlayer`)
  (set `self.SkillKey` (struct))
  (set `self.IceCoolDown` true)
  (`KismetSystemLibrary.PrintString` "쿨타임 3초 시작" true true (struct :`R` 1.0 :`G` 0.893634 :`B` 0.349146 :`A` 1.0))
  (`KismetSystemLibrary.K2_SetTimer` null "CoolDownIce" 3.0))

(fn `SpawnMeteor`
  (bind (_returnvalue_x _returnvalue_y) (`KismetMathLibrary.BreakVector` (`self.K2_GetActorLocation` (`self.AttacAreaOb`))))
  (bind (_returnvalue_x_2 _returnvalue_y_2 _returnvalue_z) (`KismetMathLibrary.BreakVector` (`self.K2_GetActorLocation` (`GameplayStatics.GetPlayerCharacter` 0))))
  (`|SpawnActorFromClass` "/Game/LHW/Skill_Resouroes/Meteor/BP_MeteorSkill.BP_MeteorSkill_C" (`KismetMathLibrary.Conv_VectorToTransform` (`KismetMathLibrary.MakeVector` _returnvalue_x _returnvalue_y _returnvalue_z)) "Undefined" "MultiplyWithRoot" null null)
  (`self.StopMovementPlayer`)
  (set `self.SkillKey` (struct))
  (set `self.MeteorCoolDown` true)
  (`KismetSystemLibrary.PrintString` "메테오 쿨타운 시작 " true true (struct :`R` 1.0 :`G` 0.956113 :`B` 0.286401 :`A` 1.0))
  (`KismetSystemLibrary.K2_SetTimer` null "CoolDownTeteor" 6.0))

(fn `StartMovementPlayer`
  (`self.EnableInput` (`GameplayStatics.GetPlayerController` 0) null)
  (set `self.asdnalsnd` true))

(fn `StopMovementPlayer`
  (set `self.isSkillCasting` true)
  (`MovementComponent.StopMovementImmediately` (`self.CharacterMovement`))
  (`self.DisableInput` (`GameplayStatics.GetPlayerController` 0) null)
  (set `self.asdnalsnd` false))

(fn `UserConstructionScript`)